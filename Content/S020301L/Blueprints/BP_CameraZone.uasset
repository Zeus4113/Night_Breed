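; BP_CameraZone is a trigger volume that blends a character's camera spring arm to a zone-specific length while inside.
; On Box overlap by an IBP_Char actor, it stores the character and its current arm length, then plays a Timeline lerping toward NewCameraLength.
; Leaving reverses the Timeline back to the stored length, which is re-captured on every entry, even mid-blend.
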(event `self.Box.OnComponentBeginOverlap`
  (params (OverlappedComponent :type "PrimitiveComponent Object Reference") (OtherActor :type "Actor Object Reference") (OtherComp :type "PrimitiveComponent Object Reference") (OtherBodyIndex :type Integer) (bFromSweep :type Boolean) (SweepResult :type "HitResult Structure (by ref)"))
  (bind _asibp_char (cast `/Game/Blueprints/Character/IBP_Char` OtherActor))
  (bind _output_get (set `self.Character` _asibp_char))
  (bind _target_arm_length (`/Game/Blueprints/Character/IBP_Char.GetSpringArm` _output_get))
  (set `self.DefaultCameraLength` _target_arm_length)
  (bind (_direction _newtrack_0) (`Timeline|Timeline` :!label _label)
    (:`Update`
      (`/Game/Blueprints/Character/IBP_Char.SetSpringArm` (`self.Character`) (`KismetMathLibrary.Lerp` (`self.DefaultCameraLength`) (`self.NewCameraLength`) _newtrack_0)))))

(event `self.Box.OnComponentEndOverlap`
  (params (OverlappedComponent :type "PrimitiveComponent Object Reference") (OtherActor :type "Actor Object Reference") (OtherComp :type "PrimitiveComponent Object Reference") (OtherBodyIndex :type Integer))
  (cast `/Game/Blueprints/Character/IBP_Char` OtherActor)
  (goto _label :!via `Reverse`))

(fn `UserConstructionScript`)