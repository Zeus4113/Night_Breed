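; BP_Hook is an interactable hook point that pulls a character toward itself.
; Interact casts the interacting character to IBP_Char and launches it at a fixed speed along the direction from its location to the hook, adding to its current velocity.
; Highlight swaps the cube's material between a blue ethereal look and a door material.
; The event graph and construction script hold no logic.
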(fn `Highlight`
  (params (IsTrue :type Boolean))
  (bind _cube (`self.Cube`))
  (if IsTrue
    (`PrimitiveComponent.SetMaterial` _cube 0 "/Game/S020301L/Materials/M_BlueEthereal_2.M_BlueEthereal_2")
    (else
      (`PrimitiveComponent.SetMaterial` _cube 0 "/Game/IBGL/Environments/Misc/Exo_Deco02/Materials/M_Decos_Door.M_Decos_Door"))))

(fn `Interact`
  (params (`Interacting Character` :type "Pawn Object Reference"))
  (bind _asibp_char (cast `/Game/Blueprints/Character/IBP_Char` `Interacting Character`))
  (`Character.LaunchCharacter` _asibp_char (* (`KismetMathLibrary.GetDirectionUnitVector` (`self.K2_GetActorLocation` _asibp_char) (`self.K2_GetActorLocation`)) 1400.0) false false))

(fn `UserConstructionScript`)