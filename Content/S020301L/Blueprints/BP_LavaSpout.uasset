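; BP_LavaSpout is a lava spout hazard that can be toggled by interaction.
; Its capsule applies environmental damage when an actor implementing the IBP_Char character type begins overlapping it.
; Interact alternates through a FlipFlop, first switching off both particle systems and the capsule collision, then switching them back on at the next call.
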(event `self.Capsule.OnComponentBeginOverlap`
  (params (OverlappedComponent :type "PrimitiveComponent Object Reference") (OtherActor :type "Actor Object Reference") (OtherComp :type "PrimitiveComponent Object Reference") (OtherBodyIndex :type Integer) (bFromSweep :type Boolean) (SweepResult :type "HitResult Structure (by ref)"))
  (bind _asibp_char (cast `/Game/Blueprints/Character/IBP_Char` OtherActor))
  (`GameplayStatics.ApplyDamage` _asibp_char (`self.Damage`) null null "/Engine/EngineDamageTypes/DmgTypeBP_Environmental.DmgTypeBP_Environmental_C"))

(event `/Game/S020301L/Blueprints/BPI_Interactable.Interact`
  (bind _particlesystem1 (`self.ParticleSystem1`))
  (bind _particlesystem (`self.ParticleSystem`))
  (bind _capsule (`self.Capsule`))
  (`/Engine/EditorBlueprintResources/StandardMacros.FlipFlop`
    (:`A`
      (`ActorComponent.SetActive` _particlesystem1 false false)
      (`ActorComponent.SetActive` _particlesystem false false)
      (`PrimitiveComponent.SetCollisionEnabled` _capsule "NoCollision"))
    (:`B`
      (`ActorComponent.SetActive` _particlesystem1 true false)
      (`ActorComponent.SetActive` _particlesystem true false)
      (`PrimitiveComponent.SetCollisionEnabled` _capsule "QueryAndPhysics"))))

(fn `UserConstructionScript`)