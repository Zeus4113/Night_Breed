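; BP_Mover is an interactable actor that slides once from its current position to an offset position.
; Interact, while not yet complete, records the start location and plays the Move timeline, lerping the actor by the TriggeredMovement offset without sweeping.
; IsComplete is only set when the timeline finishes, after which further interactions are ignored.
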(event `/Game/S020301L/Blueprints/BPI_Interactable.Interact`
  (bind _start_location (`self.Start Location`))
  (if (not (`self.IsComplete`))
    (set `self.Start Location` (`self.K2_GetActorLocation`))
    (bind (_direction _rotate_float) (`Timeline|Move`)
      (:`Update`
        (`self.K2_SetActorLocation` (`KismetMathLibrary.VLerp` _start_location (+ (`self.Triggered Movement`) _start_location) _rotate_float)))
      (:`Finished`
        (set `self.IsComplete` true)))))

(fn `UserConstructionScript`)