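; Base Blueprint for level activators, with placeholder Activate and ResetActivator functions meant for child overrides.
; When interaction is enabled, CanInteract fires Activate through a DoOnce with a particle burst, and one-shot activators switch off their prompt particle.
; MultishotActivate re-arms the DoOnce, and CanResetObject optionally resets the activator on death.
; The construction script shows the prompt particle only for interactable activators, offsets it and aligns the burst to it.
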(event `/Game/Blueprints/Library/CanInteract.CanInteract`
  (params (CharacterRef :type "/Game/Blueprints/Character/IBP_Char Object Reference"))
  (if (`self.ActiveOnInteract?`)
    (`/Engine/EditorBlueprintResources/StandardMacros.DoOnce` false :!label _label
      (:`Completed`
        (`self.Activate`) ; Override
        (`ActorComponent.Activate` (`self.Action_Particle_Burst`) false)
        (if (`self.OneShot?`)
          (`ActorComponent.Deactivate` (`self.Action_Particle`)))))))

(event `MultishotActivate`
  (goto _label :!via `Reset`))

(event `/Game/Blueprints/Library/CanResetObject.CanResetObject`
  (if (`self.ResetOnDeath?`)
    (`self.ResetActivator`) ; Override
    (if (`self.ActiveOnInteract?`)
      (`ActorComponent.SetActive` (`self.Action_Particle`) true true)
      (`self.MultishotActivate`))))

(fn `Activate`
  (returns (Complete :type Boolean))
  (return true))

(fn `ResetActivator`
  (returns (complete :type Boolean))
  (return false))

(fn `UserConstructionScript`
  (bind (_actioniconoffset_x _actioniconoffset_y _actioniconoffset_z) (`KismetMathLibrary.BreakVector` (`self.ActionIconOffset`)))
  (`SceneComponent.SetVisibility` (`self.Action_Particle`) (`self.ActiveOnInteract?`) true)
  (`SceneComponent.K2_AddRelativeLocation` (`self.Action_Particle`) (`KismetMathLibrary.MakeVector` _actioniconoffset_x _actioniconoffset_y _actioniconoffset_z) false false)
  (`SceneComponent.K2_SetWorldLocation` (`self.Action_Particle_Burst`) (`SceneComponent.K2_GetComponentLocation` (`self.Action_Particle`)) false false))