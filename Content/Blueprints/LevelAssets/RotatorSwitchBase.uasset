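; Base rotating lever switch, a child of an interactable switch class, that swings its RotatePoint in pitch when interacted with.
; The construction script sets the starting pitch from InitialPitch, then a timeline lerps it toward GoToPitch.
; Unless OneShot is set, the timeline reverses on finishing, with a DoOnce re-armed on each pull to prevent looping.
; ResetSwitch restores the initial rotation and rewinds the timeline.
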(event `PullLever`
  (bind _initialrotation (`self.InitialRotation`))
  (`self.ResetPlayback`)
  (bind (_direction _alphatrack) (`Timeline|TL_PullLever` :!label _label)
    (:`Update`
      (`SceneComponent.K2_SetRelativeRotation` (`self.RotatePoint`) (`KismetMathLibrary.MakeRotator` 0.0 (.pitch (`KismetMathLibrary.RLerp` _initialrotation (`KismetMathLibrary.MakeRotator` (.roll _initialrotation) (`self.GoToPitch`) (.yaw _initialrotation)) _alphatrack))) false false))
    (:`Finished`
      (if (not (`self.OneShot?`))
        (`/Engine/EditorBlueprintResources/StandardMacros.DoOnce` false :!label _label_2
          (:`Completed`
            (`self.PlaybackTL`)))))))

(event `PlaybackTL`
  (goto _label :!via `Reverse`))

(event `ResetTimeline`
  (goto _label :!via `SetNewTime`))

(event `ResetPlayback`
  (goto _label_2 :!via `Reset`))

(event `self.ReceiveBeginPlay`)

(fn `InteractFunctionality`
  (returns (Complete :type Boolean))
  (bind _complete (`parent.InteractFunctionality`))
  (`self.PullLever`)
  (return _complete))

(fn `ResetSwitch`
  (returns (Complete :type Boolean))
  (bind _complete (`parent.ResetSwitch`))
  (`SceneComponent.K2_SetWorldRotation` (`self.RotatePoint`) (`self.InitialRotation`) false false)
  (`self.ResetTimeline`)
  (return _complete))

(fn `UserConstructionScript`
  (bind (_returnvalue_roll _returnvalue_pitch _returnvalue_yaw) (`KismetMathLibrary.BreakRotator` (`SceneComponent.K2_GetComponentRotation` (`self.RotatePoint`))))
  (`parent.UserConstructionScript`)
  (`SceneComponent.K2_SetWorldRotation` (`self.RotatePoint`) (`KismetMathLibrary.MakeRotator` _returnvalue_roll (* (`self.InitialPitch`) -1.0) _returnvalue_yaw) false false)
  (bind _output_get (set `self.InitialRotation` (`SceneComponent.K2_GetComponentRotation` (`self.RotatePoint`))))
  (`SceneComponent.K2_SetRelativeRotation` (`self.RotatePoint`) (`KismetMathLibrary.MakeRotator` 0.0 (.pitch _output_get)) false false))