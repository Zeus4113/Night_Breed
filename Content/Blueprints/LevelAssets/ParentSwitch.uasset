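; ParentSwitch is a base interactable switch whose subclasses override InteractFunctionality and ResetSwitch to define their behaviour.
; Interaction passes a DoOnce, runs the override, fires a burst particle and signals every SignalList entry, then either hides the prompt particle (OneShot) or re-arms.
; With ResetOnDeath set, CanResetObject restores and re-arms it.
; The construction script offsets the particles and can draw signal connection lines.
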(event `/Game/Blueprints/Library/CanInteract.CanInteract`
  (params (CharacterRef :type "/Game/Blueprints/Character/IBP_Char Object Reference"))
  (`/Engine/EditorBlueprintResources/StandardMacros.DoOnce` false :!label _label
    (:`Completed`
      (`self.InteractFunctionality`) ; Override
      (`ActorComponent.Activate` (`self.Action_Particle_Burst`) false)
      (for _array_element (`self.SignalList`)
        (message `/Game/Blueprints/Library/CanSignal.CanSignal` _array_element))
      (if (`self.OneShot?`)
        (`ActorComponent.Deactivate` (`self.Action_Particle`))
        (else
          (`self.MultishotActivate`))))))

(event `MultishotActivate`
  (goto _label :!via `Reset`))

(event `/Game/Blueprints/Library/CanResetObject.CanResetObject`
  (if (`self.ResetOnDeath?`)
    (`self.ResetSwitch`) ; Override
    (`self.MultishotActivate`)
    (`ActorComponent.Activate` (`self.Action_Particle`) false)))

(fn `InteractFunctionality`
  (returns (Complete :type Boolean))
  (return true))

(fn `ResetSwitch`
  (returns (Complete :type Boolean))
  (return true))

(fn `UserConstructionScript`
  (bind (_action_icon_offset_x _action_icon_offset_y _action_icon_offset_z) (`KismetMathLibrary.BreakVector` (`self.Action_Icon_Offset`)))
  (`SceneComponent.K2_AddRelativeLocation` (`self.Action_Particle`) (`KismetMathLibrary.MakeVector` _action_icon_offset_x _action_icon_offset_y _action_icon_offset_z) false false)
  (`SceneComponent.K2_SetWorldLocation` (`self.Action_Particle_Burst`) (`SceneComponent.K2_GetComponentLocation` (`self.Action_Particle`)) false false)
  (if (`self.ShowConnections`)
    (`/Game/Blueprints/Library/MacroLibrary.showSignalLines` (`self.SignalList`)
      (:`End`
        (set `self.ShowConnections` false)))))