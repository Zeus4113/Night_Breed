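; Base trigger volume that fires when a character implementing IBP_Char enters its box, sized and offset in the construction script.
; The first overlap calls the overridable Activate with the player's location, then runs UseSimple on linked simple objects and Activate on linked triggers.
; One-shot triggers then disable collision, while others re-arm after a delay.
; With ResetOnDeath, CanResetObject re-enables the trigger and calls the overridable ResetFunctionality.
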(event `self.CollisionBox.OnComponentBeginOverlap`
  (params (OverlappedComponent :type "PrimitiveComponent Object Reference") (OtherActor :type "Actor Object Reference") (OtherComp :type "PrimitiveComponent Object Reference") (OtherBodyIndex :type Integer) (bFromSweep :type Boolean) (SweepResult :type "HitResult Structure (by ref)"))
  (bind _asibp_char (cast `/Game/Blueprints/Character/IBP_Char` OtherActor))
  (`/Engine/EditorBlueprintResources/StandardMacros.DoOnce` false :!label _label
    (:`Completed`
      (`self.Activate` (`self.K2_GetActorLocation` _asibp_char)) ; Override
      (`|ExecutionSequence`
        (:`then_0`
          (for _array_element (`self.SimpleObjectList`)
            (`/Game/Blueprints/LevelAssets/ParentSimple.UseSimple` _array_element)))
        (:`then_1`
          (for _array_element_2 (`self.TriggerObjectList`)
            (`/Game/Blueprints/LevelAssets/ParentActivater.Activate` _array_element_2))
          (if (`self.OneShot?`)
            (`self.SwitchIO` false)
            (else
              (`KismetSystemLibrary.Delay` (`self.ReactivateDelay`))
              (`self.MultishotActivate`))))))))

(event `MultishotActivate`
  (goto _label :!via `Reset`))

(event `SwitchIO`
  (params (`On?` :type Boolean))
  (bind _collisionbox (`self.CollisionBox`))
  (if `On?`
    (`PrimitiveComponent.SetCollisionEnabled` _collisionbox "QueryOnly")
    (else
      (`PrimitiveComponent.SetCollisionEnabled` _collisionbox "NoCollision"))))

(event `/Game/Blueprints/Library/CanResetObject.CanResetObject`
  (if (`self.ResetOnDeath?`)
    (`self.SwitchIO` true)
    (`self.MultishotActivate`)
    (`self.ResetFunctionality`)))

(fn `Activate`
  (params (PlayerLocation :type "Vector Structure"))
  (returns (Complete :type Boolean))
  (return true))

(fn `ResetFunctionality`
  (returns (complete :type Boolean))
  (return true))

(fn `UserConstructionScript`
  (bind _collisionbox (`self.CollisionBox`))
  (`BoxComponent.SetBoxExtent` _collisionbox (`self.CollisionBoxScale`) true)
  (`SceneComponent.K2_SetRelativeLocation` _collisionbox (`self.CollisionOffset`) false false))