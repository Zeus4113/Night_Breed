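; RoomCam01 is a per-room camera actor that becomes the view target, with a short blend, when IBP_Char overlaps its trigger box.
; Its construction script sets the box extent, spring arm rotation and length, camera centre offset, and a plane sized to the room.
; When Follow is enabled, Tick moves a billboard component to the player's X and Z position, clamped to bounds derived from room centre and size.
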(event `self.ReceiveBeginPlay`
  (bind _asibp_char (cast `/Game/Blueprints/Character/IBP_Char` (`GameplayStatics.GetPlayerPawn` 0)))
  (set `self.IBPCharREF` _asibp_char))

(event `self.ReceiveTick`
  (params (DeltaSeconds :type "Float (single-precision)"))
  (bind (_returnvalue_x _returnvalue_y _returnvalue_z) (`KismetMathLibrary.BreakVector` (`self.K2_GetActorLocation`)))
  (bind (_roomcentre_x _roomcentre_y _roomcentre_z) (`KismetMathLibrary.BreakVector` (`self.RoomCentre`)))
  (bind (_returnvalue_x_2 _returnvalue_y_2 _returnvalue_z_2) (`KismetMathLibrary.BreakVector` (`self.K2_GetActorLocation` (`self.IBPCharREF`))))
  (bind _returnvalue (* (`self.RooxZ`) 50.0))
  (bind _returnvalue_2 (* (`self.RoomX`) 50.0))
  (if (`self.Follow`)
    (`SceneComponent.K2_SetWorldLocation` (`self.MaterialBillboard`) (`KismetMathLibrary.MakeVector` (`KismetMathLibrary.FClamp` _returnvalue_x_2 (- (+ _roomcentre_x _returnvalue_x) _returnvalue_2) (+ (+ _returnvalue_x _roomcentre_x) _returnvalue_2)) 0.0 (`KismetMathLibrary.FClamp` _returnvalue_z_2 (- (+ _roomcentre_z _returnvalue_z) _returnvalue) (+ (+ _roomcentre_z _returnvalue_z) _returnvalue))) false false)))

(event `self.Box.OnComponentBeginOverlap`
  (params (OverlappedComponent :type "PrimitiveComponent Object Reference") (OtherActor :type "Actor Object Reference") (OtherComp :type "PrimitiveComponent Object Reference") (OtherBodyIndex :type Integer) (bFromSweep :type Boolean) (SweepResult :type "HitResult Structure (by ref)"))
  (cast `/Game/Blueprints/Character/IBP_Char` OtherActor)
  (`PlayerController.SetViewTargetWithBlend` (`GameplayStatics.GetPlayerController` 0) self 0.5 "VTBlend_Linear" 0.5 false))

(fn `UserConstructionScript`
  (bind _springarm (`self.SpringArm`))
  (`BoxComponent.SetBoxExtent` (`self.Box`) (`self.In Box Extent`) true)
  (`SceneComponent.K2_SetWorldRotation` _springarm (`self.Rotate`) false false)
  (set `SpringArmComponent.TargetArmLength` (`self.SpringLength`) _springarm)
  (`SceneComponent.K2_AddLocalOffset` (`self.MaterialBillboard`) (`self.CamCentre`) false false)
  (`SceneComponent.SetWorldScale3D` (`self.Plane`) (`KismetMathLibrary.MakeVector` (`self.RoomX`) (`self.RooxZ`) 1.0))
  (`SceneComponent.K2_AddLocalOffset` (`self.Plane`) (`self.RoomCentre`) false false))