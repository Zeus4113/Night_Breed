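; CamRig01 is a placeable camera rig that blends the player's view to itself when an IBP_Char enters its trigger box.
; The construction script applies instance settings for box size, spring arm rotation and length, and a centre offset on the MaterialBillboard.
; Each tick, optional Follow moves the billboard to the player character's location, and optional RotateFollow aims the camera at that character.
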(event `self.ReceiveBeginPlay`
  (bind _asibp_char (cast `/Game/Blueprints/Character/IBP_Char` (`GameplayStatics.GetPlayerPawn` 0)))
  (set `self.As IBP Char` _asibp_char))

(event `self.ReceiveTick`
  (params (DeltaSeconds :type "Float (single-precision)"))
  (`|ExecutionSequence`
    (:`then_0`
      (if (`self.Follow`)
        (`SceneComponent.K2_SetWorldLocation` (`self.MaterialBillboard`) (`self.K2_GetActorLocation` (`self.As IBP Char`)) false false)))
    (:`then_1`
      (if (`self.RotateFollow`)
        (`SceneComponent.K2_SetWorldRotation` (`self.Camera`) (`KismetMathLibrary.FindLookAtRotation` (`SceneComponent.K2_GetComponentLocation` (`self.Camera`)) (`self.K2_GetActorLocation` (`self.As IBP Char`))) false false)))))

(event `self.Box.OnComponentBeginOverlap`
  (params (OverlappedComponent :type "PrimitiveComponent Object Reference") (OtherActor :type "Actor Object Reference") (OtherComp :type "PrimitiveComponent Object Reference") (OtherBodyIndex :type Integer) (bFromSweep :type Boolean) (SweepResult :type "HitResult Structure (by ref)"))
  (cast `/Game/Blueprints/Character/IBP_Char` OtherActor)
  (`PlayerController.SetViewTargetWithBlend` (`GameplayStatics.GetPlayerController` 0) self 0.5 "VTBlend_Linear" 0.5 false))

(fn `UserConstructionScript`
  (bind _springarm (`self.SpringArm`))
  (`BoxComponent.SetBoxExtent` (`self.Box`) (`self.In Box Extent`) true)
  (`SceneComponent.K2_SetWorldRotation` _springarm (`self.Rotate`) false false)
  (set `SpringArmComponent.TargetArmLength` (`self.SpringLength`) _springarm)
  (`SceneComponent.K2_AddLocalOffset` (`self.MaterialBillboard`) (`self.CamCentre`) false false))