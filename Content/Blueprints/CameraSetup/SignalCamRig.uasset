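; Trigger-volume camera rig that blends the player's view to itself when the player character enters its box, optionally tracking the character's position or aim.
; A one-shot signal switches it to a second "GOTO" setup of follow modes, rotation and centre, with a timeline lerping spring arm length.
; The construction script applies both setups to separate components.
; A reset event optionally restores the initial setup on player death.
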(event `self.ReceiveBeginPlay`
  (bind _asibp_char (cast `/Game/Blueprints/Character/IBP_Char` (`GameplayStatics.GetPlayerPawn` 0)))
  (set `self.As IBP Char` _asibp_char))

(event `self.ReceiveTick`
  (params (DeltaSeconds :type "Float (single-precision)"))
  (`|ExecutionSequence`
    (:`then_0`
      (if (`self.HoldFollow`)
        (`SceneComponent.K2_SetWorldLocation` (`self.MaterialBillboard`) (`self.K2_GetActorLocation` (`self.As IBP Char`)) false false)))
    (:`then_1`
      (if (`self.HoldFollowRotate`)
        (`SceneComponent.K2_SetWorldRotation` (`self.Camera`) (`KismetMathLibrary.FindLookAtRotation` (`SceneComponent.K2_GetComponentLocation` (`self.Camera`)) (`self.K2_GetActorLocation` (`self.As IBP Char`))) false false)))))

(event `self.Box.OnComponentBeginOverlap`
  (params (OverlappedComponent :type "PrimitiveComponent Object Reference") (OtherActor :type "Actor Object Reference") (OtherComp :type "PrimitiveComponent Object Reference") (OtherBodyIndex :type Integer) (bFromSweep :type Boolean) (SweepResult :type "HitResult Structure (by ref)"))
  (cast `/Game/Blueprints/Character/IBP_Char` OtherActor)
  (`PlayerController.SetViewTargetWithBlend` (`GameplayStatics.GetPlayerController` 0) self 0.5 "VTBlend_Linear" 0.5 false))

(event `/Game/Blueprints/Library/CanSignal.CanSignal`
  (bind _springarm (`self.SpringArm`))
  (bind _gotofollow (`self.GOTOFollow`))
  (bind _gotofollowrotate (`self.GOTOFollowRotate`))
  (`/Engine/EditorBlueprintResources/StandardMacros.DoOnce` false :!label _label
    (:`Completed`
      (set `self.HoldFollow` _gotofollow)
      (set `self.HoldFollowRotate` _gotofollowrotate)
      (`SceneComponent.K2_SetWorldRotation` _springarm (`self.GOTORotate`) false false)
      (`SceneComponent.K2_SetRelativeLocation` (`self.MaterialBillboard`) (`self.GOTOCamCentre`) false false)
      (if (and (== _gotofollow false) (== _gotofollowrotate false))
        (`SceneComponent.K2_SetRelativeRotation` :`self` (`self.Camera`))
        (bind (_direction _newtrack_0) (`Timeline|SpringArmGOTO` :!via `PlayFromStart` :!label _label_2)
          (:`Update`
            (set `SpringArmComponent.TargetArmLength` (`KismetMathLibrary.Lerp` (`self.SpringLength`) (`self.GOTOSpringLength`) _newtrack_0) _springarm)))
        (else
          (goto _label_2 :!via `PlayFromStart`))))))

(event `/Game/Blueprints/Library/CanResetObject.CanResetObject`
  (bind _springarm (`self.SpringArm`))
  (if (`self.ResetOnPlayerDeath`)
    (`|ExecutionSequence`
      (:`then_0`
        (goto _label :!via `Reset`))
      (:`then_1`
        (`SceneComponent.K2_SetWorldRotation` _springarm (`self.Rotate`) false false)
        (set `SpringArmComponent.TargetArmLength` (`self.SpringLength`) _springarm)
        (`SceneComponent.K2_SetRelativeLocation` (`self.MaterialBillboard`) (`self.CamCentre`) false false)
        (set `self.HoldFollow` (`self.Follow`))
        (set `self.HoldFollowRotate` (`self.RotateFollow`))))))

(fn `UserConstructionScript`
  (bind _springarm (`self.SpringArm`))
  (`|ExecutionSequence`
    (:`then_0`
      (`BoxComponent.SetBoxExtent` (`self.Box`) (`self.In Box Extent`) true)
      (`SceneComponent.K2_SetWorldRotation` _springarm (`self.Rotate`) false false)
      (set `SpringArmComponent.TargetArmLength` (`self.SpringLength`) _springarm)
      (`SceneComponent.K2_AddLocalOffset` (`self.MaterialBillboard`) (`self.CamCentre`) false false)
      (set `self.HoldFollow` (`self.Follow`))
      (set `self.HoldFollowRotate` (`self.RotateFollow`)))
    (:`then_1`
      (`SceneComponent.K2_SetWorldRotation` (`self.GOTOSPRING`) (`self.GOTORotate`) false false)
      (`SceneComponent.K2_AddLocalOffset` (`self.GOTOCenre`) (`self.GOTOCamCentre`) false false)
      (set `SpringArmComponent.TargetArmLength` (`self.GOTOSpringLength`) (`self.GOTOSPRING`)))))