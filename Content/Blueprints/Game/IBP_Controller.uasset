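; Player controller for a side-scrolling action character, handling input, spawning and RPG progression.
; On start it teleports the pawn to a checkpoint or PlayerStart, then adds the HUD and a play-time timer.
; Input drives movement, attacks, double-tap dodges and slides, using timers and CanAttack/CanDodge gates.
; LevelStatsStruct holds stats for XP leveling, the inventory widget, throw costs paid in Hearts, and recharging mana.
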(event `InputAction|TimeSLow`
  (params (Key :type "Key Structure"))
  (:`Pressed`
    (`GameplayStatics.SetGlobalTimeDilation` 0.5))
  (:`Released`
    (`GameplayStatics.SetGlobalTimeDilation` 1.0)))

(event `/Game/Blueprints/LevelAssets/SoundManager/SoundManagerInterface.SetupSoundManagerReference`
  (params (SoundManagerReference :type "/Game/Blueprints/LevelAssets/SoundManager/SoundManager Object Reference"))
  ;[1 1 1] Setup Sound Manager, this is done via the Game Mode Class
  (set `self.SoundManager` SoundManagerReference))

(event `Block Input`
  (`/Engine/EditorBlueprintResources/StandardMacros.FlipFlop`
    (:`A`
      (`self.DisableInput` null))
    (:`B`
      (`self.DisableInput` null))))

(event `self.ReceiveBeginPlay`
  ;[1 1 1] Spawn
  (`KismetSystemLibrary.Delay` 0.2)
  (`self.SpawnCharacter`))

(event `SpawnCharacter`
  (bind _asibp_char (cast `/Game/Blueprints/Character/IBP_Char` (`self.K2_GetPawn`) :!pure true))
  (bind _checkpointactor (`/Game/Blueprints/Character/IBP_Char.CheckPointActor` _asibp_char))
  ;[1 1 1] InitiationChain
  (`/Engine/EditorBlueprintResources/StandardMacros.IsValid` _checkpointactor
    (:`Is Valid`
      (set `/Game/Blueprints/Character/IBP_Char.ShouldPlayOpeningCinematic` false _asibp_char)
      (`self.K2_TeleportTo` :`self` _asibp_char :`DestLocation` (`self.K2_GetActorLocation` _checkpointactor))
      (bind _output_get (set `self.IBPCharREF` _asibp_char :!label _label))
      (`self.Possess` _output_get)
      (bind _returnvalue (`|CreateWidget` "/Game/Blueprints/HUD/GameHUD.GameHUD_C" self (`self.IBPCharREF`)))
      (bind _output_get_2 (set `self.GameHUDREF` _returnvalue))
      (`UserWidget.AddToViewport` _output_get_2 0)
      (`KismetSystemLibrary.K2_SetTimer` null "AddToTime" 1.0 true)
      (set `/Game/Blueprints/Character/IBP_Char.ControllerRef` self (`self.IBPCharREF`))
      (set `/Game/Blueprints/Character/IBP_Char.SoundManager` (`self.SoundManager`) (`self.IBPCharREF`)))
    (:`Is Not Valid`
      (bind _outactors (`GameplayStatics.GetAllActorsOfClass` "/Script/Engine.PlayerStart"))
      (for _array_element _outactors
        (`self.K2_TeleportTo` :`self` _asibp_char :`DestLocation` (`self.K2_GetActorLocation` _array_element))
        (goto _label)))))

(event `Key|I`
  (params (Key :type "Key Structure"))
  (bind (_levelstatsstruct_strength _levelstatsstruct_defense _levelstatsstruct_intelligence _levelstatsstruct_luck _levelstatsstruct_level _levelstatsstruct_currentxp _levelstatsstruct_mpmax _levelstatsstruct_mp _levelstatsstruct_hearts _levelstatsstruct_playername _levelstatsstruct_kills _levelstatsstruct_gold _levelstatsstruct_nextxp _levelstatsstruct_maxhearts _levelstatsstruct_timeseconds _levelstatsstruct_timeminutes _levelstatsstruct_timehours _levelstatsstruct_hp _levelstatsstruct_hpmax) (break `/Game/Blueprints/Library/LevelStats` (`self.LevelStatsStruct`)))
  ;[1 1 1] Show Stats / Inventory
  (:`Pressed`
    (if (`self.IsInventoryOpen`)
      (`Widget.RemoveFromParent` (`self.InventoryRef`))
      (set `self.IsInventoryOpen` false)
      (else
        (bind _returnvalue (`|CreateWidget` "/Game/Blueprints/HUD/Inventory.Inventory_C" self))
        (bind _output_get (set `self.InventoryRef` _returnvalue))
        (`UserWidget.AddToViewport` _output_get 0)
        (set `self.IsInventoryOpen` true)
        (`self.UpdateUI` _levelstatsstruct_strength _levelstatsstruct_defense _levelstatsstruct_intelligence _levelstatsstruct_luck _levelstatsstruct_level _levelstatsstruct_currentxp _levelstatsstruct_mpmax _levelstatsstruct_mp _levelstatsstruct_hearts _levelstatsstruct_playername _levelstatsstruct_kills _levelstatsstruct_gold _levelstatsstruct_nextxp _levelstatsstruct_maxhearts _levelstatsstruct_hp _levelstatsstruct_hpmax)))))

(event `InputAction|Crouch`
  (params (Key :type "Key Structure"))
  (bind _ibpcharref (`self.IBPCharREF`))
  ;[0 1 0] Character Crouch
  (:`Pressed`
    (if (!= (`Character.CanJump` (`GameplayStatics.GetPlayerCharacter` 0)) false)
      (`Character.Crouch` _ibpcharref)
      (`/Game/Blueprints/Character/IBP_Char.CrouchCamOffset` _ibpcharref true)))
  (:`Released`
    (`Character.UnCrouch` _ibpcharref)
    (`/Game/Blueprints/Character/IBP_Char.CrouchCamOffset` _ibpcharref false)))

(event `InputAction|Interaction`
  (params (Key :type "Key Structure"))
  ;[0 1 0] Interact
  (:`Pressed`
    (`/Game/Blueprints/Character/IBP_Char.EventInteract` (`self.IBPCharREF`))))

(event `self.ReceiveTick`
  (params (DeltaSeconds :type "Float (single-precision)"))
  ;[1 1 1] Fake XP Generation
)

(event `Key|LeftBracket`
  (params (Key :type "Key Structure"))
  (:`Pressed`
    (`KismetSystemLibrary.ExecuteConsoleCommand` "HighResShot 2" self)))

(event `Key|RightBracket`
  (params (Key :type "Key Structure"))
  ;[1 1 1] Fake XP Generation
  (:`Pressed`
    (`self.GainXP` 100.0)))

(event `IncrementKills`
  (bind (_levelstatsstruct_strength _levelstatsstruct_defense _levelstatsstruct_intelligence _levelstatsstruct_luck _levelstatsstruct_level _levelstatsstruct_currentxp _levelstatsstruct_mpmax _levelstatsstruct_mp _levelstatsstruct_hearts _levelstatsstruct_playername _levelstatsstruct_kills) (break `/Game/Blueprints/Library/LevelStats` (`self.LevelStatsStruct`)))
  ;[1 1 1] Increase Score Kills
  (`/Engine/EditorBlueprintResources/StandardMacros.IncrementFloat` _levelstatsstruct_kills))

(event `InputAction|MeleeAttack`
  (params (Key :type "Key Structure"))
  ;[1 1 1] Attack Input and Ammo Check
  (:`Pressed`
    (if (`self.CanAttack`)
      (set `self.CanAttack` false)
      (set `self.canDodge` false)
      (`/Game/Blueprints/Character/IBP_Char.MeleeAttackSet` (`self.IBPCharREF`))))
  (:`Released`
    (`/Game/Blueprints/Character/IBP_Char.MeleeAttackUnset` (`self.IBPCharREF`))))

(event `InputAction|ThrowAttack`
  (params (Key :type "Key Structure"))
  ;[1 1 1] Attack Input and Ammo Check
  (:`Pressed`
    (if (`self.CanAttack`)
      (bind _hasammo (`self.CheckThrowAmmo`))
      (if _hasammo
        (set `self.CanAttack` false)
        (set `self.canDodge` false)
        (`/Game/Blueprints/Character/IBP_Char.ThrowAttackSet` (`self.IBPCharREF`)))))
  (:`Released`
    (`/Game/Blueprints/Character/IBP_Char.ThrowAttackUnset` (`self.IBPCharREF`))))

(event `InputAxis|MoveCharacter`
  (params (AxisValue :type "Float (single-precision)"))
  ;[1 0 0] Left Right Movement
  (if (not (== AxisValue 0.0))
    (if (> AxisValue 0.0)
      (`self.SetControlRotation` (`self.Right`))
      (else
        (`self.SetControlRotation` (`self.Left`))))
    (`Pawn.AddMovementInput` (`self.K2_GetPawn`) (1.0 0.0 0.0) AxisValue false)))

(event `InputAction|MagicAttack`
  (params (Key :type "Key Structure"))
  ;[1 1 1] Attack Input and Ammo Check
  (:`Pressed`
    (if (`self.CanAttack`)
      (bind _hasammo (`self.CheckMagicAmmo`))
      (if _hasammo
        (set `self.CanAttack` false)
        (set `self.canDodge` false)
        (`/Game/Blueprints/Character/IBP_Char.MagicAttackSet` (`self.IBPCharREF`)))))
  (:`Released`
    (`/Game/Blueprints/Character/IBP_Char.MagicAttackUnset` (`self.IBPCharREF`))))

(event `InputAction|DodgeRight`
  (params (Key :type "Key Structure"))
  (:`Pressed`
    (if (== (`self.LastInput`) 0)
      (set `self.LastInput` 1)
      (`KismetSystemLibrary.K2_SetTimerDelegate` (delegate `ClearDoubleTap`) 0.2 :!label _label_2)
      (elif (== (`self.LastInput`) 1)
        (set `self.LastInput` 0)
        ;[1 1 1] Slide and Dodge Mechanics
        (if (`self.canDodge`)
          (`KismetSystemLibrary.K2_SetTimerDelegate` (delegate `ClearDodgeCount`) (`self.DodgeDectTime`))
          (`/Engine/EditorBlueprintResources/StandardMacros.IncrementInt` (`self.DodgeCount`)
            (:`  `
              (if (not (>= (`self.DodgeCount`) 2))
                (`self.Dodge` (1500.0 0.0 0.0))
                (set `self.CanAttack` false)
                (set `self.canDodge` false)
                (`KismetSystemLibrary.K2_SetTimerDelegate` (delegate `DodgeRecharge`) (`self.DodgeReset`))
                (`/Game/Blueprints/LevelAssets/SoundManager/SoundManager.PlaySFX` (`self.SoundManager`) "/Game/Sounds/GregSourced/Whoosh2_Cue.Whoosh2_Cue" (`self.K2_GetActorLocation` (`self.IBPCharREF`)))))))))))

(event `ReplenishMana`
  (bind (_levelstatsstruct_strength _levelstatsstruct_defense _levelstatsstruct_intelligence _levelstatsstruct_luck _levelstatsstruct_level _levelstatsstruct_currentxp _levelstatsstruct_mpmax _levelstatsstruct_mp) (break `/Game/Blueprints/Library/LevelStats` (`self.LevelStatsStruct`)))
  ;[1 1 1] Recharge Mana Over Time
  (if (< _levelstatsstruct_mp _levelstatsstruct_mpmax)
    (bind _returnvalue (`KismetSystemLibrary.K2_SetTimerDelegate` (delegate `AddToMana`) (`self.ManaRechargeSpeed`) true))
    (set `self.ManaRechargeTimer` _returnvalue)
    (else
      (`KismetSystemLibrary.K2_ClearAndInvalidateTimerHandle` (`self.ManaRechargeTimer`)))))

(event `InputAction|DodgeLeft`
  (params (Key :type "Key Structure"))
  (:`Pressed`
    (if (== (`self.LastInput`) 0)
      (set `self.LastInput` 2)
      (goto _label_2)
      (elif (== (`self.LastInput`) 2)
        (set `self.LastInput` 0)
        ;[1 1 1] Slide and Dodge Mechanics
        (if (`self.canDodge`)
          (`KismetSystemLibrary.K2_SetTimerDelegate` (delegate `ClearDodgeCount`) (`self.DodgeDectTime`))
          (`/Engine/EditorBlueprintResources/StandardMacros.IncrementInt` (`self.DodgeCount`)
            (:`  `
              (if (not (>= (`self.DodgeCount`) 2))
                (`self.Dodge` (-1500.0 0.0 0.0))
                (set `self.CanAttack` false)
                (set `self.canDodge` false)
                (`KismetSystemLibrary.K2_SetTimerDelegate` (delegate `DodgeRecharge`) (`self.DodgeReset`))
                (`/Game/Blueprints/LevelAssets/SoundManager/SoundManager.PlaySFX` (`self.SoundManager`) "/Game/Sounds/GregSourced/Whoosh2_Cue.Whoosh2_Cue" (`self.K2_GetActorLocation` (`self.IBPCharREF`)))))))))))

(event `DodgeRecharge`
  (bind _charactermovement (`Character.CharacterMovement` (`GameplayStatics.GetPlayerCharacter` 0)))
  ;[1 1 1] Slide and Dodge Mechanics
  (set `self.canDodge` true)
  (set `self.CanAttack` true)
  (set `CharacterMovementComponent.GroundFriction` 1.0 _charactermovement)
  (set `CharacterMovementComponent.FallingLateralFriction` 1.0 _charactermovement))

(event `ClearDodgeCount`
  ;[1 1 1] Slide and Dodge Mechanics
  (set `self.DodgeCount` 0))

(event `ClearDoubleTap`
  (set `self.LastInput` 0))

(event `AddToMana`
  (bind (_levelstatsstruct_strength _levelstatsstruct_defense _levelstatsstruct_intelligence _levelstatsstruct_luck _levelstatsstruct_level _levelstatsstruct_currentxp _levelstatsstruct_mpmax _levelstatsstruct_mp) (break `/Game/Blueprints/Library/LevelStats` (`self.LevelStatsStruct`)))
  ;[1 1 1] Recharge Mana Over Time
  (setmembers `/Game/Blueprints/Library/LevelStats` :`StructRef` (`self.LevelStatsStruct`) :`Mp` (`KismetMathLibrary.Conv_IntToDouble` (`KismetMathLibrary.FFloor` (`KismetMathLibrary.FClamp` (+ _levelstatsstruct_mp (+ (/ _levelstatsstruct_intelligence 100.0) (`self.ManaRechargeAmount`))) 0.0 _levelstatsstruct_mpmax))))
  (`self.ReplenishMana`))

(event `InputAction|Slide`
  (params (Key :type "Key Structure"))
  ;[1 1 1] Slide and Dodge Mechanics
  (:`Pressed`
    (if (and (`self.canDodge`) (!= (`/Game/Blueprints/Character/IBP_Char.isInAir` (cast `/Game/Blueprints/Character/IBP_Char` (`self.K2_GetPawn`) :!pure true)) true))
      (`KismetSystemLibrary.K2_SetTimerDelegate` (delegate `ClearDodgeCount`) (`self.DodgeDectTime`))
      (`/Engine/EditorBlueprintResources/StandardMacros.IncrementInt` (`self.DodgeCount`)
        (:`  `
          (if (== (`self.DodgeCount`) 2)
            (`self.CrouchSlide` (* (`self.GetActorForwardVector` (`self.K2_GetPawn`)) (1500.0 0.0 0.0)))
            (set `self.CanAttack` false)
            (set `self.canDodge` false)
            (`KismetSystemLibrary.K2_SetTimerDelegate` (delegate `DodgeRecharge`) (`self.DodgeReset`))
            (`/Game/Blueprints/LevelAssets/SoundManager/SoundManager.PlaySFX` (`self.SoundManager`) "/Game/Sounds/GregSourced/Whoosh2_Cue.Whoosh2_Cue" (`self.K2_GetActorLocation` (`self.IBPCharREF`)))))))))

(event `InputAction|Jump`
  (params (Key :type "Key Structure"))
  ;[1 1 1] Trigger Jump
  (:`Pressed`
    (`/Game/Blueprints/Character/IBP_Char.TriggerJump` (`self.IBPCharREF`))))

(event `Dodge`
  (params (Dir :type "Vector Structure"))
  (bind _returnvalue (`GameplayStatics.GetPlayerCharacter` 0))
  (bind _charactermovement (`Character.CharacterMovement` _returnvalue))
  ;[1 1 1] Dodge
  (set `CharacterMovementComponent.GroundFriction` 0.0 _charactermovement)
  (set `CharacterMovementComponent.FallingLateralFriction` 0.0 _charactermovement)
  (set `MovementComponent.Velocity` Dir _charactermovement)
  (`AnimInstance.Montage_Play` (cast `/Game/PlayerCharacter/Vampire/VampireBlueprint` (`SkeletalMeshComponent.GetAnimInstance` (`Character.Mesh` (cast `/Game/Blueprints/Character/IBP_Char` _returnvalue :!pure true))) :!pure true) "/Game/PlayerCharacter/Vampire/DodgeMontage.DodgeMontage" 1.0 "MontageLength" 0.0 true))

(event `CrouchSlide`
  (params (Dir :type "Vector Structure"))
  (bind _returnvalue (`GameplayStatics.GetPlayerCharacter` 0))
  (bind _charactermovement (`Character.CharacterMovement` _returnvalue))
  ;[1 1 1] Crouch Slide
  (set `CharacterMovementComponent.GroundFriction` 0.0 _charactermovement)
  (set `CharacterMovementComponent.FallingLateralFriction` 0.0 _charactermovement)
  (set `MovementComponent.Velocity` Dir _charactermovement)
  (`AnimInstance.Montage_Play` (cast `/Game/PlayerCharacter/Vampire/VampireBlueprint` (`SkeletalMeshComponent.GetAnimInstance` (`Character.Mesh` (cast `/Game/Blueprints/Character/IBP_Char` _returnvalue :!pure true))) :!pure true) "/Game/PlayerCharacter/Vampire/SlideMontage.SlideMontage" 1.0 "MontageLength" 0.0 true))

(fn `AddToTime`
  (bind (_levelstatsstruct_strength _levelstatsstruct_defense _levelstatsstruct_intelligence _levelstatsstruct_luck _levelstatsstruct_level _levelstatsstruct_currentxp _levelstatsstruct_mpmax _levelstatsstruct_mp _levelstatsstruct_hearts _levelstatsstruct_playername _levelstatsstruct_kills _levelstatsstruct_gold _levelstatsstruct_nextxp _levelstatsstruct_maxhearts _levelstatsstruct_timeseconds) (break `/Game/Blueprints/Library/LevelStats` (`self.LevelStatsStruct`)))
  (bind (_levelstatsstruct_strength_2 _levelstatsstruct_defense_2 _levelstatsstruct_intelligence_2 _levelstatsstruct_luck_2 _levelstatsstruct_level_2 _levelstatsstruct_currentxp_2 _levelstatsstruct_mpmax_2 _levelstatsstruct_mp_2 _levelstatsstruct_hearts_2 _levelstatsstruct_playername_2 _levelstatsstruct_kills_2 _levelstatsstruct_gold_2 _levelstatsstruct_nextxp_2 _levelstatsstruct_maxhearts_2 _levelstatsstruct_timeseconds_2 _levelstatsstruct_timeminutes) (break `/Game/Blueprints/Library/LevelStats` (`self.LevelStatsStruct`)))
  (bind (_levelstatsstruct_strength_3 _levelstatsstruct_defense_3 _levelstatsstruct_intelligence_3 _levelstatsstruct_luck_3 _levelstatsstruct_level_3 _levelstatsstruct_currentxp_3 _levelstatsstruct_mpmax_3 _levelstatsstruct_mp_3 _levelstatsstruct_hearts_3 _levelstatsstruct_playername_3 _levelstatsstruct_kills_3 _levelstatsstruct_gold_3 _levelstatsstruct_nextxp_3 _levelstatsstruct_maxhearts_3 _levelstatsstruct_timeseconds_3 _levelstatsstruct_timeminutes_2 _levelstatsstruct_timehours) (break `/Game/Blueprints/Library/LevelStats` (`self.LevelStatsStruct`)))
  ;[1 1 1] Increase time by first adding to seconds, then incrementing minutes and finally increasing hours
  (bind _result (`/Engine/EditorBlueprintResources/StandardMacros.IncrementInt` _levelstatsstruct_timeseconds)
    (:`  `
      (if (>= _result 60)
        (setmembers `/Game/Blueprints/Library/LevelStats` :`StructRef` (`self.LevelStatsStruct`) :`TimeSeconds` 0)
        (bind _result_2 (`/Engine/EditorBlueprintResources/StandardMacros.IncrementInt` _levelstatsstruct_timeminutes)
          (:`  `
            (if (>= _result_2 60)
              (setmembers `/Game/Blueprints/Library/LevelStats` :`StructRef` (`self.LevelStatsStruct`) :`TimeMinutes` 0)
              (`/Engine/EditorBlueprintResources/StandardMacros.IncrementInt` _levelstatsstruct_timehours
                (:`  `
                  (return)))
              (else
                (return)))))
        (else
          (return))))))

(fn `CheckLevelUp`
  (bind (_levelstatsstruct_strength _levelstatsstruct_defense _levelstatsstruct_intelligence _levelstatsstruct_luck) (break `/Game/Blueprints/Library/LevelStats` (`self.LevelStatsStruct`)))
  (bind (_strength _defense _intelligence _luck _level _currentxp _mpmax _mp _hearts _playername _kills _gold _nextxp) (break `/Game/Blueprints/Library/LevelStats` (`self.LevelStatsStruct`)))
  ;[1 1 1] Check if XP is equal to the required XP for the next level and if so level up
  (if (>= _currentxp _nextxp)
    (`/Engine/EditorBlueprintResources/StandardMacros.IncrementFloat` _level
      (:`  `
        ;[1 1 1] Work out XP for next level and play VFX for leveling
        (`self.CheckXPforNextLevel`)
        (`self.PlayLevelUpEffects`)
        ;[1 1 1] Increase Character Stats for leveling
        (`/Game/Blueprints/Library/LevellingLibrary.LevelIncrement` _levelstatsstruct_strength 10.0
          (:`  `
            (`/Game/Blueprints/Library/LevellingLibrary.LevelIncrement` _levelstatsstruct_defense 10.0
              (:`  `
                (`/Game/Blueprints/Library/LevellingLibrary.LevelIncrement` _levelstatsstruct_intelligence 10.0
                  (:`  `
                    (`/Game/Blueprints/Library/LevellingLibrary.LevelIncrement` _levelstatsstruct_luck 10.0
                      (:`  `
                        (return)))))))))))
    (else
      (return))))

(fn `CheckMagicAmmo`
  (returns (HasAmmo :type Boolean))
  (bind (_levelstatsstruct_strength _levelstatsstruct_defense _levelstatsstruct_intelligence _levelstatsstruct_luck _levelstatsstruct_level _levelstatsstruct_currentxp _levelstatsstruct_mpmax _levelstatsstruct_mp) (break `/Game/Blueprints/Library/LevelStats` (`self.LevelStatsStruct`)))
  ;[1 1 1] This is a check and reduction system for Magic Ammo
  (if (>= _levelstatsstruct_mp 5.0)
    (setmembers `/Game/Blueprints/Library/LevelStats` :`StructRef` (`self.LevelStatsStruct`) :`Mp` (- _levelstatsstruct_mp 5.0))
    (`self.ReplenishMana`)
    (return true)
    (else
      (return false))))

(fn `CheckThrowAmmo`
  (returns (HasAmmo :type Boolean))
  (bind (_levelstatsstruct_strength _levelstatsstruct_defense _levelstatsstruct_intelligence _levelstatsstruct_luck _levelstatsstruct_level _levelstatsstruct_currentxp _levelstatsstruct_mpmax _levelstatsstruct_mp _levelstatsstruct_hearts) (break `/Game/Blueprints/Library/LevelStats` (`self.LevelStatsStruct`)))
  ;[1 1 1] This is a check and reduction system for Throw Ammo
  (if (>= _levelstatsstruct_hearts 5.0)
    (setmembers `/Game/Blueprints/Library/LevelStats` :`StructRef` (`self.LevelStatsStruct`) :`Hearts` (- _levelstatsstruct_hearts 5.0))
    (return true)
    (else
      (return false))))

(fn `CheckXPforNextLevel`
  (returns (XPRequired :type "Float (double-precision)"))
  (bind (_levelstatsstruct_strength _levelstatsstruct_defense _levelstatsstruct_intelligence _levelstatsstruct_luck _levelstatsstruct_level) (break `/Game/Blueprints/Library/LevelStats` (`self.LevelStatsStruct`)))
  (bind _returnvalue (* (`KismetMathLibrary.Square` _levelstatsstruct_level) 1000.0))
  ;[1 1 1] For Level 2 onwards set required by taking squaring current level and multiplying by 1000
  (setmembers `/Game/Blueprints/Library/LevelStats` :`StructRef` (`self.LevelStatsStruct`) :`NextXP` _returnvalue)
  (return _returnvalue))

(fn `GainXP`
  (params (Experience :type "Float (double-precision)"))
  (bind (_levelstatsstruct_strength _levelstatsstruct_defense _levelstatsstruct_intelligence _levelstatsstruct_luck _levelstatsstruct_level _levelstatsstruct_currentxp) (break `/Game/Blueprints/Library/LevelStats` (`self.LevelStatsStruct`)))
  ;[1 1 1] Add to Total XP and check if character is ready to level up
  (setmembers `/Game/Blueprints/Library/LevelStats` :`StructRef` (`self.LevelStatsStruct`) :`CurrentXP` (+ Experience _levelstatsstruct_currentxp))
  (`self.CheckLevelUp`)
  (return))

(fn `PlayLevelUpEffects`
  (`/Game/Blueprints/LevelAssets/SoundManager/SoundManager.PlaySFX` (`self.SoundManager`) "/Game/Sounds/GregSourced/Mana_Pickup_Cue.Mana_Pickup_Cue" (`self.K2_GetActorLocation` (`GameplayStatics.GetPlayerCharacter` 0)))
  (`/Game/Blueprints/Character/IBP_Char.LevelUpEffectStart` (`self.IBPCharREF`))
  (return))

(fn `UserConstructionScript`)