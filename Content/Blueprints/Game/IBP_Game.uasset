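; IBP_Game is a game-level Blueprint that wires up sound manager references and runs the game-over sequence.
; On BeginPlay it finds the SoundManager actor and passes it to every actor implementing SoundManagerInterface through an interface message.
; GameEnd removes all widgets, puts the first player controller into cinematic mode with movement and turning disabled, then plays the GameOverCinematic level sequence.
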(event `self.ReceiveBeginPlay`
  ;[1 1 1] On Begin Play setup sound manager reference that need it
  (bind _outactors (`GameplayStatics.GetAllActorsOfClass` "/Game/Blueprints/LevelAssets/SoundManager/SoundManager.SoundManager_C"))
  (for _array_element _outactors
    (set `self.SoundManagerRef` _array_element))
  (bind _outactors_2 (`GameplayStatics.GetAllActorsWithInterface` "/Game/Blueprints/LevelAssets/SoundManager/SoundManagerInterface.SoundManagerInterface_C"))
  (for _array_element_2 _outactors_2
    (message `/Game/Blueprints/LevelAssets/SoundManager/SoundManagerInterface.SetupSoundManagerReference` _array_element_2 (`self.SoundManagerRef`))))

(event `GameEnd`
  ;[1 1 1] Setup end level cinematic
  (`WidgetLayoutLibrary.RemoveAllWidgets`)
  (`PlayerController.SetCinematicMode` (`GameplayStatics.GetPlayerController` 0) true true true true true)
  (bind (_outactor _returnvalue) (`LevelSequencePlayer.CreateLevelSequencePlayer` "/Game/Blueprints/LevelAssets/Cinematic/GameOverCinematic.GameOverCinematic" (make `MovieSceneSequencePlaybackSettings` 0)))
  (`LevelSequencePlayer.Play` _returnvalue))

(fn `UserConstructionScript`)