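; Blueprint function library of tabletop-style dice rolls and checks.
; Roll functions fill an array with random results, then loop over it for sum, lowest, highest, average or a pass against a difficulty.
; Other helpers detect D6 pairs, critical ranges and fumbles, which roll an extra D6.
; Get2ndHighestDiceRoll forces two or more dice, but its remove-maximum step is disconnected, so it does not reliably return the second highest.
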(fn GetSumOfRolls
  (params (Rolls :type Integer) (Dice%20Sides :type Integer))
  ;[1 1 1] Add random dice rolls to array
  (for _index (range 1 Rolls)
    (Utilities|Array|Add (LocalVariables|GetDiceReturn) (Math|Random|RandomIntegerinRange 1 Dice%20Sides)))
  ;[1 1 1] Add at dice rolls together
  (for _array_element (LocalVariables|GetDiceReturn)
    (LocalVariables|SetSum (+ _array_element (LocalVariables|GetSum))))
  (return (LocalVariables|GetSum)))

(fn GetLowestDiceRoll
  (params (Rolls :type Integer) (Dice%20Sides :type Integer))
  ;[1 1 1] Add random dice rolls to array
  (for _index (range 1 Rolls)
    (Utilities|Array|Add (LocalVariables|GetDiceReturn) (Math|Random|RandomIntegerinRange 1 Dice%20Sides)))
  ;[1 1 1] Find lowest dice roll by looking through an array and comparing index to Min int
  (LocalVariables|SetMinInt (Utilities|Array|Get(acopy) (LocalVariables|GetDiceReturn)))
  (for _array_element (LocalVariables|GetDiceReturn)
    (Math|Integer|CompareInt _array_element (LocalVariables|GetMinInt)
      (:<
        (LocalVariables|SetMinInt _array_element))))
  (return (LocalVariables|GetMinInt)))

(fn GetHighestDiceRoll
  (params (Rolls :type Integer) (DiceSides :type Integer))
  ;[1 1 1] Add random dice rolls to array
  (for _index (range 1 Rolls)
    (Utilities|Array|Add (LocalVariables|GetDiceReturn) (Math|Random|RandomIntegerinRange 1 DiceSides)))
  ;[1 1 1] Look through array and compare current indexs against maximum integer, set new maximum if greater than max int
  (LocalVariables|SetMaxInt (Utilities|Array|Get(acopy) (LocalVariables|GetDiceReturn)))
  (for _array_element (LocalVariables|GetDiceReturn)
    (Math|Integer|CompareInt _array_element (LocalVariables|GetMaxInt)
      (:>
        (LocalVariables|SetMaxInt _array_element))))
  (return (LocalVariables|GetMaxInt)))

(fn GetAverageDiceRoll
  (params (Rolls :type Integer) (DiceSides :type Integer))
  ;[1 1 1] Add dice roll results to an array and calculate total
  (for _index (range 1 Rolls)
    (Utilities|Array|Add (LocalVariables|GetDiceReturn) (Math|Random|RandomIntegerinRange 1 DiceSides)))
  (for _array_element (LocalVariables|GetDiceReturn)
    (LocalVariables|SetAverage (+ _array_element (LocalVariables|GetAverage))))
  ;[1 1 1] Calculate average by dividing total by dice rolls
  (LocalVariables|SetAverage (/ (LocalVariables|GetAverage) Rolls))
  (return (LocalVariables|GetAverage)))

(fn Get2ndHighestDiceRoll
  (params (Rolls :type Integer) (DiceSides :type Integer))
  ;[1 1 1] Ensure that 2 dice are always rolled, even if the designer accidently enters 1
  (if (< Rolls 2)
    (LocalVariables|SetRollAmount 2)
    (else
      (bind _output_get (LocalVariables|SetRollAmount Rolls))))
  (for _index (range 1 _output_get)
    ;[1 1 1] Generate Random number within sides of dice limit and add to array
    (Utilities|Array|Add (LocalVariables|GetDiceReturn) (Math|Random|RandomIntegerinRange 1 DiceSides)))
  ;[1 1 1] Find Maximum roll
  (LocalVariables|SetMaxInt (Utilities|Array|Get(acopy) (LocalVariables|GetDiceReturn)))
  (for _array_element (LocalVariables|GetDiceReturn)
    (Math|Integer|CompareInt _array_element (LocalVariables|GetMaxInt)
      (:>
        (LocalVariables|SetMaxInt _array_element))))
  ;[1 1 1] Remove maximum roll from array
  (Utilities|Array|RemoveItem (LocalVariables|GetDiceReturn) 0)
  (LocalVariables|SetMaxInt 0)
  ;[1 1 1] Find second highest and return value
  (for _array_element_2 (LocalVariables|GetDiceReturn)
    (Math|Integer|CompareInt _array_element_2 (LocalVariables|GetMaxInt)
      (:>
        (LocalVariables|SetMaxInt _array_element_2))))
  (return (LocalVariables|GetMaxInt)))

(fn DifficultyPassRoll
  (params (Rolls :type Integer) (DiceSides :type Integer) (Difficulty :type Integer))
  ;[1 1 1] Add random dice rolls to array
  (for _index (range 1 Rolls)
    (Utilities|Array|Add (LocalVariables|GetDiceReturn) (Math|Random|RandomIntegerinRange 1 DiceSides)))
  ;[1 1 1] Add at dice rolls together
  (for _array_element (LocalVariables|GetDiceReturn)
    (bind _output_get (LocalVariables|SetSum (+ _array_element (LocalVariables|GetSum)))))
  ;[1 1 1] Is the total Greater than or equal to the difficult to pass this challenge
  (if (>= _output_get Difficulty)
    (return true)
    (else
      (return false))))

(fn D6PairsCheckRoll
  (bind _dicereturn (LocalVariables|GetDiceReturn))
  (bind _item (Utilities|Array|Get(acopy) _dicereturn 1))
  (bind _item_2 (Utilities|Array|Get(acopy) _dicereturn))
  ;[1 1 1] Roll 2D6
  (for _index (range 1 2)
    (Utilities|Array|Add (LocalVariables|GetDiceReturn) (Math|Random|RandomIntegerinRange 1 6)))
  ;[1 1 1] Work out outputs
  (return _item_2 (== _item_2 _item) (+ _item_2 _item)))

(fn CriticalCheck
  (params (TotalInput :type Integer) (CriticalMin :type Integer) (CriticalHigh :type Integer))
  ;[1 1 1] See if a roll score is within a critical region
  (return (Math|Float|InRange(Float) (Math|Conversions|ToFloat(Integer) TotalInput) (Math|Conversions|ToFloat(Integer) CriticalMin) (Math|Conversions|ToFloat(Integer) CriticalHigh))))

(fn FumbleCheck
  (params (DiceResult :type Integer))
  ;[1 1 1] Check Dice score against a 1, if Score is equal to one then roll a D6, the resultant roll can be used to determine what happens on a fumble, if you do not fumble the output is always 0 i.e. worthless
  (if (== DiceResult 1)
    (return true (Math|Random|RandomIntegerinRange 1 6))
    (else
      (return false 0))))