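; Patrol enemy that walks back and forth between two points and hurts the player on touch, with no other AI.
; The construction script offsets both points from the capsule in X and Z and moves marker components there.
; From BeginPlay, MoveToAndSwitch starts an AI move, flips Direction immediately, and calls itself again on success.
; HitPlayer runs the parent logic, then calls MoveToAndSwitch to reverse the patrol.
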(event `self.ReceiveBeginPlay`
  ;[1 1 1] As soon as the game starts this enemy patrols
  (`self.MoveToAndSwitch`))

(event `MoveToAndSwitch`
  ;[1 1 1] This enemy patrols between two vectors set. It hurts the player on touch but has no other AI
  (if (`self.Direction`)
    (`|AIMoveTo` self (`self.PatrolLocationLeft`)
      (:`then`
        (set `self.Direction` false))
      (:`OnSuccess`
        (`self.MoveToAndSwitch` :!label _label)))
    (else
      (`|AIMoveTo` self (`self.PatrolLocationRight`)
        (:`then`
          (set `self.Direction` true))
        (:`OnSuccess`
          (goto _label))))))

(fn `HitPlayer`
  (params (CharacterIn :type "/Game/Blueprints/Character/IBP_Char Object Reference"))
  (returns (Complete :type Boolean))
  ;[1 1 1] If we hit a player reverse the patrol
  (bind _complete (`parent.HitPlayer` CharacterIn))
  (`self.MoveToAndSwitch`)
  (return _complete))

(fn `UserConstructionScript`
  (bind (_returnvalue_x _returnvalue_y _returnvalue_z) (`KismetMathLibrary.BreakVector` (`SceneComponent.K2_GetComponentLocation` (`self.CapsuleComponent`))))
  ;[1 1 1] Determine the patrol vectors, this is done by looking at how far the distance of Width and Height variables are from the capsule component. Deth is not taken into account as most of the gameplay occurs on a 2D Plane / Y = 0
  (`parent.UserConstructionScript`)
  (`|ExecutionSequence`
    (:`then_0`
      (bind _output_get (set `self.PatrolLocationLeft` (`KismetMathLibrary.MakeVector` (- _returnvalue_x (`self.PatrolDistanceLeft`)) _returnvalue_y (+ _returnvalue_z (`self.PatrolHeightLeft`)))))
      (`SceneComponent.K2_SetWorldLocation` (`self.PatrolPointL`) _output_get false false))
    (:`then_1`
      (bind _output_get_2 (set `self.PatrolLocationRight` (`KismetMathLibrary.MakeVector` (+ (`self.PatrolDistanceRight`) _returnvalue_x) _returnvalue_y (+ (`self.PatrolHeightRight`) _returnvalue_z))))
      (`SceneComponent.K2_SetWorldLocation` (`self.PatrolPointR`) _output_get_2 false false))))