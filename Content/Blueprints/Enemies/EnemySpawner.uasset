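; Trigger-volume enemy spawner that spawns BaseEnemy actors when the player character enters its collision volume while active.
; SpawnEnemy re-arms itself on a timer to spawn up to SpawnAmount enemies with a delay between each, then deactivates once it runs again at the limit.
; EnableCollision re-activates it, and CanResetObject also clears the count for reuse.
; The construction script lets designers position the spawn point and trigger per instance.
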(event `EnableCollision`
  (set `self.isActive` true))

(event `self.CollisionTrigger.OnComponentBeginOverlap`
  (params (OverlappedComponent :type "PrimitiveComponent Object Reference") (OtherActor :type "Actor Object Reference") (OtherComp :type "PrimitiveComponent Object Reference") (OtherBodyIndex :type Integer) (bFromSweep :type Boolean) (SweepResult :type "HitResult Structure (by ref)"))
  ;[1 1 1] When the player touches the collision volume spawn the enemies, this could be done another way, experiment :-D
  (if (`self.isActive`)
    (cast `/Game/Blueprints/Character/IBP_Char` OtherActor)
    (`self.Spawn Enemy`)))

(event `Spawn Enemy`
  ;[1 1 1] Spawn enemy and increment amount spawn if more than one demanded
  (if (< (`self.CurrentSpawned`) (`self.SpawnAmount`))
    (`|SpawnActorFromClass` (`self.BaseEnemy`) (`SceneComponent.K2_GetComponentToWorld` (`self.SpawnLocation`)) "AlwaysSpawn" "OverrideRootScale" null null null)
    (`/Engine/EditorBlueprintResources/StandardMacros.IncrementInt` (`self.CurrentSpawned`)
      (:`  `
        (if (> (`self.SpawnAmount`) 1)
          (`KismetSystemLibrary.K2_SetTimerDelegate` (delegate `Spawn Enemy`) (`self.DelayBetweenSpawn`)))))
    (else
      (set `self.isActive` false))))

(event `/Game/Blueprints/Library/CanResetObject.CanResetObject`
  ;[1 1 1] On reset reduce amount spawned to 0
  (set `self.CurrentSpawned` 0)
  (set `self.isActive` true))

(fn `UserConstructionScript`
  ;[1 1 1] Allow designers to customise the location of the spawning and the trigger volume
  (`SceneComponent.K2_SetRelativeLocation` (`self.SpawnLocation`) (`self.SpawnLoc`) false false)
  (`SceneComponent.K2_SetRelativeLocation` (`self.CollisionTrigger`) (`self.CollisionLocation`) false false))