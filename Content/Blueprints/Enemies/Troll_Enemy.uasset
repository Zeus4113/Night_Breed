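; Troll boss enemy that spawns hidden, plays a timed entrance montage, then starts its AI controller.
; Club overlaps, toggled by collision, damage and launch player characters; hits on the troll update boss HUD health and grant brief invulnerability.
; A countdown enables the smash montage, with timers resetting smash state and later signalling BombSpawners.
; Lethal damage triggers the death animation, while the Death event ends the game through the game mode.
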(event `self.WeaponCollision.OnComponentBeginOverlap`
  (params (OverlappedComponent :type "PrimitiveComponent Object Reference") (OtherActor :type "Actor Object Reference") (OtherComp :type "PrimitiveComponent Object Reference") (OtherBodyIndex :type Integer) (bFromSweep :type Boolean) (SweepResult :type "HitResult Structure (by ref)"))
  ;[1 1 1] Apply force and damage on club swings
  (bind _asibp_char (cast `/Game/Blueprints/Character/IBP_Char` OtherActor))
  (`self.LaunchCharacter` _asibp_char (* (* (`KismetMathLibrary.GetForwardVector` (`self.GetControlRotation`)) -1.0) (`self.ClubKnockBack`)) true true)
  (`GameplayStatics.ApplyDamage` _asibp_char (`self.ClubDamage`))
  (`self.ToggleClubCollision` false))

(event `self.ReceiveAnyDamage`
  (params (Damage :type "Float (single-precision)") (DamageType :type "DamageType Object Reference") (InstigatedBy :type "Controller Object Reference") (DamageCauser :type "Actor Object Reference"))
  (bind _returnvalue (- (`self.Health`) Damage))
  (bind _gamehudref (`/Game/Blueprints/Game/IBP_Controller.GameHUDREF` (cast `/Game/Blueprints/Game/IBP_Controller` (`GameplayStatics.GetPlayerController` 0) :!pure true)))
  ;[1 1 1] On receive damage either die or play hit fx
  (bind _asfloating_damage (cast `/Game/Blueprints/HUD/FloatingDamage` (`WidgetComponent.GetUserWidgetObject` (`self.Widget`))))
  (set `/Game/Blueprints/HUD/FloatingDamage.Damage` Damage _asfloating_damage)
  (`/Game/Blueprints/HUD/FloatingDamage.Activate` _asfloating_damage)
  (set `self.DamageCauser` DamageCauser)
  (if (`self.Invun`)
    _
    (elif (<= _returnvalue 0.0)
      (`/Game/Blueprints/HUD/GameHUD.HideBossHealth` _gamehudref)
      (set `self.Dead` true)
      (`self.PlayDeath`)
      (`MovementComponent.StopMovementImmediately` (`self.CharacterMovement`))
      (else
        (set `self.Health` _returnvalue)
        (`/Game/Blueprints/HUD/GameHUD.UpdateBossHealth` _gamehudref (`self.Health`) (`self.MaxHealth`))
        (set `self.Invun` true)
        (`KismetSystemLibrary.K2_SetTimerDelegate` (delegate `CustomEvent`) 0.3)
        (`self.PlayHitFX`)))))

(event `CustomEvent`
  ;[1 1 1] On receive damage either die or play hit fx
  (set `self.Invun` false))

(event `ToggleClubCollision`
  (params (CollisionStatus :type Boolean))
  ;[1 1 1] Toggle Claw Collision
  (if CollisionStatus
    (`/Engine/EditorBlueprintResources/StandardMacros.IsValid` self
      (:`Is Valid`
        (`PrimitiveComponent.SetCollisionEnabled` (`self.WeaponCollision`) "QueryAndPhysics")))
    (else
      (`/Engine/EditorBlueprintResources/StandardMacros.IsValid` self
        (:`Is Valid`
          (`PrimitiveComponent.SetCollisionEnabled` (`self.WeaponCollision`) "NoCollision"))))))

(event `PlayDeath`
  ;[1 1 1] Set death animation
  (set `/Game/Blueprints/Enemies/TrollBoss/TrollAnimBlueprint.bDie` true (cast `/Game/Blueprints/Enemies/TrollBoss/TrollAnimBlueprint` (`SkeletalMeshComponent.GetAnimInstance` (`self.Mesh`)) :!pure true)))

(event `self.Death`
  ;[1 1 1] Trigger End of Level / Cinematic
  (`parent.Death`)
  (`/Game/Blueprints/Game/IBP_Game.GameEnd` (cast `/Game/Blueprints/Game/IBP_Game` (`GameplayStatics.GetGameMode`) :!pure true)))

(event `self.ReceiveBeginPlay`
  ;[1 1 1] Club weapon detection is turned off after spawn
  (`KismetSystemLibrary.K2_SetTimerDelegate` (delegate `UnHide`) 0.4)
  (`self.PlayAnimMontage` "/Game/Enemy/Enemy_Troll/Enemy_Troll_Poison_Animation/TrollEntrance.TrollEntrance")
  (`self.CreateGlowMaterial`)
  (`self.ToggleClubCollision` false)
  ;[1 1 1] After entrance animation has played start AI, the time of 3.125 seconds is the length of the entrance animation
  (`KismetSystemLibrary.K2_SetTimerDelegate` (delegate `StartAI`) 3.125))

(event `StartAI`
  ;[1 1 1] After entrance animation has played start AI, the time of 3.125 seconds is the length of the entrance animation
  (`/Game/Blueprints/Enemies/TrollBoss/TrollAIController.StartAI` (cast `/Game/Blueprints/Enemies/TrollBoss/TrollAIController` (`AIBlueprintHelperLibrary.GetAIController` self) :!pure true)))

(event `UnHide`
  ;[1 1 1] Starts game as hidden and then plays falling animation
  (`SceneComponent.SetHiddenInGame` (`self.Mesh`) false false)
  (`SceneComponent.SetHiddenInGame` (`self.WeaponMesh`) false false))

(event `TrollSmash`
  ;[1 1 1] Try to play troll smash animation montage
  (if (not (`self.isSmashing`))
    (`self.PlayAnimMontage` "/Game/Enemy/Enemy_Troll/Enemy_Troll_Poison_Animation/TrollSmash.TrollSmash")
    (set `self.isSmashing` true)
    (`KismetSystemLibrary.K2_SetTimerDelegate` (delegate `UpdateState`) 2.9)
    (`KismetSystemLibrary.K2_SetTimerDelegate` (delegate `TurnOffBombs`) 6.5)))

(event `UpdateState`
  ;[1 1 1] Turn off smashing state
  (set `self.CanSmash` false)
  (set `self.isSmashing` false))

(event `TurnOffBombs`
  ;[1 1 1] Stop bombs from falling
  (bind _outactors (`GameplayStatics.GetAllActorsOfClass` "/Game/Blueprints/LevelAssets/Basic/BombSpawner.BombSpawner_C"))
  (for _array_element _outactors
    (`/Game/Blueprints/LevelAssets/Basic/BombSpawner.CanResetObject` _array_element)))

(event `DecreaseCharge`
  ;[1 1 1] Decrease time until troll releases smash animation and bombs
  (bind _result (`/Engine/EditorBlueprintResources/StandardMacros.DecrementFloat` (`self.SmashChargeTime`))
    (:`  `
      (if (<= _result 0.0)
        (`KismetSystemLibrary.K2_ClearAndInvalidateTimerHandle` (`self.SmashTimerHandle`))
        (set `self.CanSmash` true)
        (set `self.SmashChargeTime` 3.0)))))

(fn `CreateGlowMaterial`
  ;[1 1 1] Create material to show glow changes when vomit is ready
  (bind _returnvalue (`PrimitiveComponent.CreateDynamicMaterialInstance` (`self.Mesh`) 0 "/Game/Enemy/Enemy_Troll/Materials/CharM_Troll_Poison.CharM_Troll_Poison" "None"))
  (bind _output_get (set `self.TrollMaterial` _returnvalue))
  (bind _returnvalue_2 (`MaterialInstanceDynamic.K2_GetScalarParameterValue` _output_get "GlowStrength"))
  (set `self.Glow` _returnvalue_2)
  (return))

(fn `GetSegmentAtTime`
  (params (StartLocation :type "Vector Structure") (IntialVelocity :type "Vector Structure") (Gravity :type "Vector Structure") (Time1 :type "Float (double-precision)") (Time2 :type "Float (double-precision)"))
  (returns (Point1 :type "Vector Structure") (Point2 :type "Vector Structure"))
  (return (+ StartLocation (* IntialVelocity Time1) (* Gravity (* Time1 Time1 0.5))) (+ StartLocation (* IntialVelocity Time2) (* Gravity (* Time2 Time2 0.5)))))

(fn `UserConstructionScript`
  (`parent.UserConstructionScript`)
  (`SceneComponent.SetHiddenInGame` (`self.Mesh`) true true))