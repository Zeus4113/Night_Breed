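; Suicide bomber enemy that stays idle until the player character enters its CollisionRange box, sized along X by ActivationRange.
; It then uses AIMoveTo toward the player's location at activation, detonating on arrival or through HitPlayer.
; Detonate spawns explosion particles and sphere-traces to apply BombDamage to a hit character capsule.
; Death follows damage or an empty trace, but is skipped when either hit cast fails.
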(event `self.CollisionRange.OnComponentBeginOverlap`
  (params (OverlappedComponent :type "PrimitiveComponent Object Reference") (OtherActor :type "Actor Object Reference") (OtherComp :type "PrimitiveComponent Object Reference") (OtherBodyIndex :type Integer) (bFromSweep :type Boolean) (SweepResult :type "HitResult Structure (by ref)"))
  ;[1 1 1] AI only enables when player has entered collision area. AI will then path toward the player
  (bind _asibp_char (cast `/Game/Blueprints/Character/IBP_Char` OtherActor))
  (`self.Activate` (`SceneComponent.K2_GetComponentLocation` (`Character.Mesh` _asibp_char))))

(event `Activate`
  (params (AttackPosition :type "Vector Structure"))
  ;[1 1 1] AI only enables when player has entered collision area. AI will then path toward the player
  (`|AIMoveTo` self (`SceneComponent.K2_GetComponentLocation` (`Character.Mesh` (stale `self.CollisionRange.OnComponentBeginOverlap` _asibp_char))) null 5.0 true
    (:`then`
      (set `self.ShouldWalk` true))
    (:`OnSuccess`
      (set `self.ShouldWalk` false)
      (`self.Detonate`))))

(event `Detonate`
  (bind _returnvalue (`self.K2_GetActorLocation`))
  ;[1 1 1] Detonation plays particles and then traces for actors to damage,  Damage is controlled by the float Bomb Damage
  (`GameplayStatics.SpawnEmitterAtLocation` "/Game/Particles/P_BomberExplode.P_BomberExplode" (- _returnvalue (0.0 0.0 85.0)))
  (bind (_outhit _returnvalue_2) (`KismetSystemLibrary.SphereTraceSingleForObjects` _returnvalue (+ _returnvalue (0.0 0.0 1.0)) 200.0 (`self.SearchArray`)))
  (if _returnvalue_2
    (bind (_bblockinghit _binitialoverlap _time _location _impactpoint _normal _impactnormal _physmat _hitactor _hitcomponent) (`GameplayStatics.BreakHitResult` _outhit))
    (bind _asibp_char (cast `/Game/Blueprints/Character/IBP_Char` _hitactor))
    (cast `CapsuleComponent` _hitcomponent)
    (`GameplayStatics.ApplyDamage` _asibp_char (`self.BombDamage`) null self))
  (`self.Death`))

(fn `HitPlayer`
  (params (CharacterIn :type "/Game/Blueprints/Character/IBP_Char Object Reference"))
  (returns (Complete :type Boolean))
  ;[1 1 1] If we hit player, call he deonate event
  (`self.Detonate`)
  (return false))

(fn `UserConstructionScript`
  ;[1 1 1] Setup AI detection, instead of using a BOX this could also be done with a perception system if you needed accurate FOV.
  (`parent.UserConstructionScript`)
  (`BoxComponent.SetBoxExtent` (`self.CollisionRange`) (`KismetMathLibrary.MakeVector` (`self.ActivationRange`) 32.0 64.0) true))