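; Floating head enemy, a flying Character that drifts along world X in a sine-wave bob and self-destructs after ten seconds.
; Tick sets its location directly, deriving height from current X around the start position cached in the Construction Script.
; Player capsule overlaps toggle its capsule's active state and call HitPlayer.
; Any damage records the causer and calls Death, which, like HitPlayer, is defined outside these graphs.
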(event `self.ReceiveTick`
  (params (DeltaSeconds :type "Float (single-precision)"))
  (bind (_vlastpos_x _vlastpos_y _vlastpos_z) (`KismetMathLibrary.BreakVector` (`self.vLastPos`)))
  ;[1 1 1] Maths formula used to created oscilating movement
  (`self.SinWaveMovement` (* DeltaSeconds (`self.X Speed`)) (`self.Wave Height`) 75.0 _vlastpos_z _vlastpos_y))

(event `self.ReceiveBeginPlay`
  ;[1 1 1] Destroy these enemies after 10 seconds and setup the movement mode
  (`KismetSystemLibrary.K2_SetTimer` self "Death" 10.0)
  (`CharacterMovementComponent.SetMovementMode` (`self.CharacterMovement`) "MOVE_Flying" 0))

(event `self.CapsuleComponent.OnComponentBeginOverlap`
  (params (OverlappedComponent :type "PrimitiveComponent Object Reference") (OtherActor :type "Actor Object Reference") (OtherComp :type "PrimitiveComponent Object Reference") (OtherBodyIndex :type Integer) (bFromSweep :type Boolean) (SweepResult :type "HitResult Structure (by ref)"))
  (bind _asibp_char (cast `/Game/Blueprints/Character/IBP_Char` OtherActor))
  (cast `CapsuleComponent` OtherComp)
  (`ActorComponent.ToggleActive` (`self.CapsuleComponent`))
  (`self.HitPlayer` _asibp_char))

(event `self.ReceiveAnyDamage`
  (params (Damage :type "Float (single-precision)") (DamageType :type "DamageType Object Reference") (InstigatedBy :type "Controller Object Reference") (DamageCauser :type "Actor Object Reference"))
  (set `self.DamageCauser` DamageCauser)
  (`self.Death`))

(fn `SinWaveMovement`
  (params (Speed :type "Float (double-precision)") (WaveHeight :type "Float (double-precision)") (WaveLength :type "Float (double-precision)") (ZStartPosition :type "Float (double-precision)") (YPosition :type "Float (double-precision)"))
  (bind _returnvalue_x (`KismetMathLibrary.BreakVector` (`self.K2_GetActorLocation`)))
  (`self.K2_SetActorLocation` (`KismetMathLibrary.MakeVector` (+ Speed _returnvalue_x) YPosition (+ (* WaveHeight (`KismetMathLibrary.Sin` (/ _returnvalue_x WaveLength))) ZStartPosition)))
  (return))

(fn `UserConstructionScript`
  (set `self.vLastPos` (`self.K2_GetActorLocation` self)))