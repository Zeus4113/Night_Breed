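; Enemy Blueprint that throws projectiles once the player character (IBP_Char) enters an activation sphere sized by ActivationRange in the construction script.
; The first matching overlap triggers Activate and Fire, which waits a random delay within the fire-frequency range, then sets the Throwing flag.
; A separate FireProj event, not called within these graphs, spawns a Base_Projectile at a randomly chosen high or low attack point, passing damage and speed.
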(event `self.Activate_Collision.OnComponentBeginOverlap`
  (params (OverlappedComponent :type "PrimitiveComponent Object Reference") (OtherActor :type "Actor Object Reference") (OtherComp :type "PrimitiveComponent Object Reference") (OtherBodyIndex :type Integer) (bFromSweep :type Boolean) (SweepResult :type "HitResult Structure (by ref)"))
  (cast `/Game/Blueprints/Character/IBP_Char` OtherActor)
  (`/Engine/EditorBlueprintResources/StandardMacros.DoOnce` false
    (:`Completed`
      (`self.Activate`))))

(event `Activate`
  (`self.Fire`))

(event `Fire`
  (`KismetSystemLibrary.Delay` (`KismetMathLibrary.RandomFloatInRange` (`self.MinFireFrequency`) (`self.MaxFireFrequency`)))
  (set `self.throwing` true))

(event `FireProj`
  (switch `int` (`KismetMathLibrary.RandomIntegerInRange` 0 1)
    (:`Default`
      (`|SpawnActorFromClass` "/Game/Blueprints/Enemies/Base/Base_Projectile.Base_Projectile_C" (`SceneComponent.K2_GetComponentToWorld` (`self.HighAttackPoint`)) "Undefined" "OverrideRootScale" null (`self.ProjectileDamage`) (`self.ProjectileSpeed`) self :!label _label))
    (:`0`
      (goto _label))
    (:`1`
      (`|SpawnActorFromClass` "/Game/Blueprints/Enemies/Base/Base_Projectile.Base_Projectile_C" (`SceneComponent.K2_GetComponentToWorld` (`self.LowAttackPoint`)) "Undefined" "OverrideRootScale" null (`self.ProjectileDamage`) (`self.ProjectileSpeed`) self))))

(fn `UserConstructionScript`
  (`parent.UserConstructionScript`)
  (`SphereComponent.SetSphereRadius` (`self.Activate_Collision`) (`self.ActivationRange`) true))