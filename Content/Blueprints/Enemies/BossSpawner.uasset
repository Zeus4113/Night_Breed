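; Boss spawner that creates a Troll_Enemy at its spawn location and resets the encounter through CanResetObject.
; SpawnEnemy passes waypoints and the first SoundManager found to the troll, deactivates the spawner and shows boss health on the HUD.
; The troll's OnDeath is bound to TrollDead, which fires BossKilled.
; CanResetObject destroys all Troll_Enemy actors, hides the boss HUD, clears the reference and reactivates the spawner.
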(event `Troll Dead`
  (`self.BossKilled`))

(event `self.Spawn Enemy`
  (bind _troll (`self.Troll`))
  (bind _gamehudref (`/Game/Blueprints/Game/IBP_Controller.GameHUDREF` (cast `/Game/Blueprints/Game/IBP_Controller` (`GameplayStatics.GetPlayerController` 0) :!pure true)))
  ;[1 1 1] Spawn a boss, setup the UI, turn off the spawner
  (bind _outactors (`GameplayStatics.GetAllActorsOfClass` "/Game/Blueprints/LevelAssets/SoundManager/SoundManager.SoundManager_C"))
  (bind _returnvalue (`|SpawnActorFromClass` "/Game/Blueprints/Enemies/Troll_Enemy.Troll_Enemy_C" (`SceneComponent.K2_GetComponentToWorld` (`self.SpawnLocation`)) "AlwaysSpawn" "OverrideRootScale" null (`self.WayPointArray`) (`|GetArrayItem` _outactors) null))
  (bind _output_get (set `self.Troll` _returnvalue))
  (add `/Game/Blueprints/Enemies/Troll_Enemy.OnDeath` _output_get (delegate `Troll Dead`))
  (set `self.isActive` false)
  (`/Game/Blueprints/HUD/GameHUD.RevealBossHealth` _gamehudref)
  (`/Game/Blueprints/HUD/GameHUD.UpdateBossHealth` _gamehudref (`/Game/Blueprints/Enemies/Base/EnemyBase.Health` _troll) (`/Game/Blueprints/Enemies/Troll_Enemy.MaxHealth` _troll)))

(event `/Game/Blueprints/Library/CanResetObject.CanResetObject`
  ;[1 1 1] If the player dies, find the boss/es and destroy them. Hide the Boss UI, null the reference to the troll, allow the boss trigger to be active so we can spawn a new one.
  (bind _outactors (`GameplayStatics.GetAllActorsOfClass` "/Game/Blueprints/Enemies/Troll_Enemy.Troll_Enemy_C"))
  (for _array_element _outactors
    (`self.K2_DestroyActor` _array_element))
  (`/Game/Blueprints/HUD/GameHUD.HideBossHealth` (`/Game/Blueprints/Game/IBP_Controller.GameHUDREF` (cast `/Game/Blueprints/Game/IBP_Controller` (`GameplayStatics.GetPlayerController` 0) :!pure true)))
  (set `self.isActive` true)
  (set `self.Troll` null))

(fn `UserConstructionScript`
  (`parent.UserConstructionScript`))