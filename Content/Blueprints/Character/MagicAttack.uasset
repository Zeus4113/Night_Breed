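; MagicAttack is a thrown magic projectile that damages enemies and breakables, playing sounds through the level's SoundManager on spawn and wall impact.
; Sphere overlap with an EnemyBase capsule applies CalculateDamage's result, the floored square of player Level plus Strength over scaled enemy defense, falling back to fixed damage when that is zero.
; BaseBreakable targets take fixed damage.
; Damaging a target or hitting a wall calls Death.
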(event `self.ReceiveBeginPlay`
  ;[1 1 1] setup sound manager references
  (`parent.ReceiveBeginPlay`)
  (bind _outactors (`GameplayStatics.GetAllActorsOfClass` "/Game/Blueprints/LevelAssets/SoundManager/SoundManager.SoundManager_C"))
  (bind _output_get (set `self.SoundManager` (`|GetArrayItem` _outactors)))
  (`/Game/Blueprints/LevelAssets/SoundManager/SoundManager.PlaySFX` _output_get (`self.MagicSpawnCue`) (`self.K2_GetActorLocation`)))

(event `self.Sphere.OnComponentBeginOverlap`
  (params (OverlappedComponent :type "PrimitiveComponent Object Reference") (OtherActor :type "Actor Object Reference") (OtherComp :type "PrimitiveComponent Object Reference") (OtherBodyIndex :type Integer) (bFromSweep :type Boolean) (SweepResult :type "HitResult Structure (by ref)"))
  (bind _returnvalue (`self.GetInstigator`))
  ;[1 1 1] Calculate and apply damage based on the target we overlap. The thrown attack damages both breakable blueprints and characters. There are 3 results that can happen a) Damage a breakable asset, b) apply 5 damage to an npc and c) apply a custom amount of damage to an npc
  (if (!= OtherActor self)
    (bind _asenemy_base (cast `/Game/Blueprints/Enemies/Base/EnemyBase` OtherActor)
      (:`then`
        (cast `CapsuleComponent` OtherComp
          (:`then`
            (bind _returndamage (`self.CalculateDamage` (`/Game/Blueprints/Enemies/Base/EnemyBase.EnemyDefense` _asenemy_base)))
            (if (> _returndamage 0.0)
              (`GameplayStatics.ApplyDamage` _asenemy_base _returndamage null _returnvalue)
              (else
                (`GameplayStatics.ApplyDamage` _asenemy_base 5.0 null _returnvalue)))
            (`self.Death`))
          (:`CastFailed`
            (bind _asbase_breakable (cast `/Game/Blueprints/LevelAssets/Breakable/BaseBreakable` OtherActor :!label _label))
            (`GameplayStatics.ApplyDamage` _asbase_breakable 5.0)
            (`self.Death`))))
      (:`CastFailed`
        (goto _label)))))

(event `self.ReceiveHit`
  (params (MyComp :type "PrimitiveComponent Object Reference") (Other :type "Actor Object Reference") (OtherComp :type "PrimitiveComponent Object Reference") (bSelfMoved :type Boolean) (HitLocation :type "Vector Structure") (HitNormal :type "Vector Structure") (NormalImpulse :type "Vector Structure") (Hit :type "HitResult Structure (by ref)"))
  ;[1 1 1] If the attack hits a wall explode
  (`/Game/Blueprints/LevelAssets/SoundManager/SoundManager.PlaySFX` (`self.SoundManager`) (`self.MagicExplodeCue`) (`self.K2_GetActorLocation`))
  (`self.Death`))

(fn `CalculateDamage`
  (params (InputDefense :type "Float (double-precision)"))
  (returns (returndamage :type "Float (double-precision)"))
  (bind _returnvalue (`GameplayStatics.GetPlayerController` 0))
  (bind (_levelstatsstruct_strength _levelstatsstruct_defense _levelstatsstruct_intelligence _levelstatsstruct_luck _levelstatsstruct_level) (break `/Game/Blueprints/Library/LevelStats` (`/Game/Blueprints/Game/IBP_Controller.LevelStatsStruct` (cast `/Game/Blueprints/Game/IBP_Controller` _returnvalue :!pure true))))
  ;[1 1 1] To figure out damage = ((Level * 10) + Strength )Squared  / EnemyDefense * 10
  (`/Engine/EditorBlueprintResources/StandardMacros.IsValid` _returnvalue
    (:`Is Valid`
      (return (`KismetMathLibrary.Conv_IntToDouble` (`KismetMathLibrary.FFloor` (/ (`KismetMathLibrary.Square` (+ _levelstatsstruct_level _levelstatsstruct_strength)) (* InputDefense 10.0))))))
    (:`Is Not Valid`
      (return 0.0))))

(fn `UserConstructionScript`
  (`parent.UserConstructionScript`))