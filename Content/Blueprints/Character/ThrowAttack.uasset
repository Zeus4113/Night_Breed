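; ThrowAttack is a thrown attack that damages enemies and breakable objects when its sphere overlaps them, then calls Death.
; EnemyBase hits register only on capsule components, using CalculateDamage with a fallback of 5 when the result is not positive.
; CalculateDamage squares the sum of player Level and Strength from the controller's stats and scales it down by enemy defense.
; BaseBreakable targets take a fixed amount of damage.
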(event `self.Sphere.OnComponentBeginOverlap`
  (params (OverlappedComponent :type "PrimitiveComponent Object Reference") (OtherActor :type "Actor Object Reference") (OtherComp :type "PrimitiveComponent Object Reference") (OtherBodyIndex :type Integer) (bFromSweep :type Boolean) (SweepResult :type "HitResult Structure (by ref)"))
  (bind _returnvalue (`self.GetInstigator`))
  ;[1 1 1] Calculate and apply damage based on the target we overlap. The thrown attack damages both breakable blueprints and characters. There are 3 results that can happen a) Damage a breakable asset, b) apply 5 damage to an npc and c) apply a custom amount of damage to an npc
  (if (!= OtherActor self)
    (bind _asenemy_base (cast `/Game/Blueprints/Enemies/Base/EnemyBase` OtherActor)
      (:`then`
        (cast `CapsuleComponent` OtherComp)
        (bind _returndamage (`self.CalculateDamage` (`/Game/Blueprints/Enemies/Base/EnemyBase.EnemyDefense` _asenemy_base)))
        (if (> _returndamage 0.0)
          (`GameplayStatics.ApplyDamage` _asenemy_base _returndamage null _returnvalue)
          (else
            (`GameplayStatics.ApplyDamage` _asenemy_base 5.0 null _returnvalue)))
        (`self.Death`))
      (:`CastFailed`
        (cast `/Game/Blueprints/LevelAssets/Breakable/BaseBreakable` OtherActor)
        (`GameplayStatics.ApplyDamage` null 5.0)
        (`self.Death`)))))

(fn `CalculateDamage`
  (params (InputDefense :type "Float (double-precision)"))
  (returns (returndamage :type "Float (double-precision)"))
  (bind _returnvalue (`GameplayStatics.GetPlayerController` 0))
  (bind (_levelstatsstruct_strength _levelstatsstruct_defense _levelstatsstruct_intelligence _levelstatsstruct_luck _levelstatsstruct_level) (break `/Game/Blueprints/Library/LevelStats` (`/Game/Blueprints/Game/IBP_Controller.LevelStatsStruct` (cast `/Game/Blueprints/Game/IBP_Controller` _returnvalue :!pure true))))
  ;[1 1 1] To figure out damage = ((Level * 10) + Strength )Squared  / EnemyDefense * 10
  (`/Engine/EditorBlueprintResources/StandardMacros.IsValid` _returnvalue
    (:`Is Valid`
      (return (`KismetMathLibrary.Conv_IntToDouble` (`KismetMathLibrary.FFloor` (/ (`KismetMathLibrary.Square` (+ _levelstatsstruct_level _levelstatsstruct_strength)) (* InputDefense 10.0))))))
    (:`Is Not Valid`
      (return 0.0))))

(fn `UserConstructionScript`
  (`parent.UserConstructionScript`))